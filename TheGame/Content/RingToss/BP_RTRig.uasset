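; BP_RTRig is the ring toss rig that detects rings landing in its scoring rows and tells each ring what that row is worth.
; On BeginPlay it binds begin and end overlap handlers to every box component under ScoreZone.
; An entering BP_Ring receives the row's score, parsed as an integer from the box's first component tag.
; A leaving ring is told to exit the score zone.
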(event `self.ReceiveBeginPlay`
  (for _array_element (`SceneComponent.GetChildrenComponents` (`self.ScoreZone`) true)
    (bind _asbox_collision (cast `BoxComponent` _array_element))
    ; Attempt Scoring
    (add `PrimitiveComponent.OnComponentBeginOverlap` _asbox_collision (delegate `BeginOverlap`))
    ; Invalidate Score
    (add `PrimitiveComponent.OnComponentEndOverlap` _asbox_collision (delegate `EndOverlap`))))

(event `BeginOverlap`
  (params (OverlappedComponent :type "PrimitiveComponent Object Reference") (OtherActor :type "Actor Object Reference") (OtherComp :type "PrimitiveComponent Object Reference") (OtherBodyIndex :type Integer) (bFromSweep :type Boolean) (SweepResult :type "HitResult Structure (by ref)"))
  ; Attempt Scoring
  (bind _asbp_ring (cast `/Game/RingToss/BP_Ring` OtherActor))
  (`/Game/RingToss/BP_Ring.Enter Score Zone` _asbp_ring (`self.Get Row Score` OverlappedComponent)))

(event `EndOverlap`
  (params (OverlappedComponent :type "PrimitiveComponent Object Reference") (OtherActor :type "Actor Object Reference") (OtherComp :type "PrimitiveComponent Object Reference") (OtherBodyIndex :type Integer))
  ; Invalidate Score
  (bind _asbp_ring (cast `/Game/RingToss/BP_Ring` OtherActor))
  (`/Game/RingToss/BP_Ring.Exit Score Zone` _asbp_ring))

(fn `Get Row Score`
  (params (Row :type "ActorComponent Object Reference"))
  (returns (ReturnValue :type Integer))
  (return (`KismetStringLibrary.Conv_StringToInt` (`KismetStringLibrary.Conv_NameToString` (`|GetArrayItem` (`ActorComponent.ComponentTags` Row))))))

(fn `UserConstructionScript`)