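; Prototype grabbable VR ring for a ring toss game that records its motion while held.
; Grab and drop events toggle a held flag, and Tick then writes linear and angular physics velocities into small rolling arrays.
; Logic to apply the averaged velocities to the ring, hide the hand and swap weapon input mapping contexts is present but unconnected, so it never runs.
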(event `self.GrabComponent.OnGrabbed`
  (set `self.isHeld` true))

(event `self.GrabComponent.OnDropped`
  (set `self.isHeld` false))

(event `self.ReceiveTick`
  (params (DeltaSeconds :type "Float (single-precision)"))
  ; Sample Velocities if Ring is Held
  (if (`self.isHeld`)
    (`self.SampleVelocities`)))

(fn `SampleVelocities`
  (bind _myring (`self.myRing`))
  (bind _flow_control (`self.Flow Control`))
  (bind _flow_control_2 (`self.Flow Control`))
  (bind _returnvalue (`PrimitiveComponent.GetPhysicsLinearVelocity` _myring "None"))
  (`KismetArrayLibrary.Array_Set` (`self.VelocityLog`) _flow_control _returnvalue)
  (`KismetArrayLibrary.Array_Set` (`self.AngularVLog`) _flow_control (`PrimitiveComponent.GetPhysicsAngularVelocityInRadians` _myring "None"))
  (if (> _flow_control_2 4)
    (set `self.Flow Control` 0)
    (else
      (`/Engine/EditorBlueprintResources/StandardMacros.IncrementInt` _flow_control_2))))

(fn `UserConstructionScript`)