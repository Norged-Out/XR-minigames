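; Controller for the VR Ring Toss minigame, showing a start button and score widget while the XR pawn is in the start zone.
; It spawns the peg rig, then supplies randomly coloured rings one at a time, ending the game shortly after the last is used.
; Scores update the widget, the game-instance minigames handler and the score report.
; Sound events use resetting DoOnce gates to suppress rapid repeats.
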(event `self.StartZone.OnComponentBeginOverlap`
  (params (OverlappedComponent :type "PrimitiveComponent Object Reference") (OtherActor :type "Actor Object Reference") (OtherComp :type "PrimitiveComponent Object Reference") (OtherBodyIndex :type Integer) (bFromSweep :type Boolean) (SweepResult :type "HitResult Structure (by ref)"))
  (cast `/Game/XRFramework/Blueprints/BP_XRPawn` OtherActor)
  (set `self.bPlayerInRange` true)
  (`SceneComponent.SetVisibility` (`self.ScoreWidget`) true false)
  (`SceneComponent.SetVisibility` (`self.StartButton`) true false))

(event `self.StartZone.OnComponentEndOverlap`
  (params (OverlappedComponent :type "PrimitiveComponent Object Reference") (OtherActor :type "Actor Object Reference") (OtherComp :type "PrimitiveComponent Object Reference") (OtherBodyIndex :type Integer))
  (cast `/Game/XRFramework/Blueprints/BP_XRPawn` OtherActor)
  (set `self.bPlayerInRange` false)
  (`SceneComponent.SetVisibility` (`self.ScoreWidget`) false false)
  (`SceneComponent.SetVisibility` (`self.StartButton`) false false))

(event `self.ReceiveBeginPlay`
  ; Start Button
  (bind _asstart_button (cast `/Game/UI/StartButton` (`WidgetComponent.GetUserWidgetObject` (`self.StartButton`))))
  (add `/Game/UI/StartButton.OnStartPressed` _asstart_button (delegate `HandleStart`))
  (`|SpawnActorFromClass` "/Game/RingToss/BP_RTRig.BP_RTRig_C" (`SceneComponent.K2_GetComponentToWorld` (`self.PegsSpawnPoint`)) "Undefined" "MultiplyWithRoot" null null))

(event `HandleStart`
  ; Start Button
  (if (not (`self.bGameActive`))
    (`self.Start Game`)))

(event `StartGameSound`
  ; Game Sounds
  (`/Engine/EditorBlueprintResources/StandardMacros.DoOnce` false :!label _label
    (:`Completed`
      (`GameplayStatics.PlaySoundAtLocation` "/Game/Audio/Begin_Game.Begin_Game" (`self.K2_GetActorLocation`) (struct) 1.0 1.0 0.0 null null null null)
      (`KismetSystemLibrary.Delay` 0.3)
      (goto _label :!via `Reset`))))

(event `EndGameSound`
  ; Game Sounds
  (`/Engine/EditorBlueprintResources/StandardMacros.DoOnce` false :!label _label_2
    (:`Completed`
      (`GameplayStatics.PlaySoundAtLocation` "/Game/Audio/Game_End.Game_End" (`self.K2_GetActorLocation`) (struct) 1.0 1.0 0.0 null null null null)
      (`KismetSystemLibrary.Delay` 0.3)
      (goto _label_2 :!via `Reset`))))

(event `SpawnSound`
  ; Game Sounds
  (`/Engine/EditorBlueprintResources/StandardMacros.DoOnce` false :!label _label_3
    (:`Completed`
      (`GameplayStatics.PlaySoundAtLocation` "/Game/Audio/SpawnSound.SpawnSound" (`self.K2_GetActorLocation`) (struct) 1.0 1.0 0.0 null null null null)
      (`KismetSystemLibrary.Delay` 0.3)
      (goto _label_3 :!via `Reset`))))

(fn `Display Message`
  (params (inText :type Text))
  (bind _aswbp_game_score (cast `/Game/UI/WBP_GameScore` (`WidgetComponent.GetUserWidgetObject` (`self.ScoreWidget`))))
  (`/Game/UI/WBP_GameScore.SetMessage` _aswbp_game_score inText))

(fn `End Game`
  (set `self.bGameActive` false)
  (`self.EndGameSound`)
  (`self.Display Message` "Game Over"))

(fn `On Ring Used`
  (set `self.bHasActiveRing` false)
  (`self.SetLifeSpan` (`self.Ring`) 10.0)
  (bind _output_get (set `self.RingsRemaining` (- (`self.RingsRemaining`) 1)))
  (if (<= _output_get 0)
    (`KismetSystemLibrary.K2_SetTimer` null "End Game" 5.0)
    (else
      (`self.Spawn Ring`))))

(fn `Spawn Ring`
  (if (and (> (`self.RingsRemaining`) 0) (not (`self.bHasActiveRing`)))
    (bind _returnvalue (`|SpawnActorFromClass` "/Game/RingToss/BP_Ring.BP_Ring_C" (`SceneComponent.K2_GetComponentToWorld` (`self.RingSpawnPoint`)) "AlwaysSpawn" "MultiplyWithRoot" null (select `int` (`KismetMathLibrary.RandomIntegerInRange` 0 2) :`0` "/Game/Assets/Rings/RingOrange.RingOrange" :`1` "/Game/Assets/Rings/RingGreen.RingGreen" :`2` "/Game/Assets/Rings/RingPurple.RingPurple" :!type "MaterialInterface Object Reference") null))
    (bind _output_get (set `self.Ring` _returnvalue))
    (add `/Game/RingToss/BP_Ring.OnScored` _output_get (`|CreateDelegate` :!event `Update Score`))
    (set `self.bHasActiveRing` true)
    (`self.SpawnSound`)))

(fn `Start Game`
  (set `self.bGameActive` true)
  (`self.StartGameSound`)
  (set `self.RingsRemaining` (`self.RingsToSpawn`))
  (set `self.TotalScore` 0)
  (`self.Spawn Ring`)
  (`self.Display Message` "Ring Toss")
  (bind _asbp_minigames_handler (cast `/Game/Core/BP_Minigames_Handler` (`GameplayStatics.GetGameInstance`)))
  (`/Game/Core/BP_Minigames_Handler.Submit Attempt` _asbp_minigames_handler "NewEnumerator3")
  (bind _returnvalue (`GameplayStatics.GetActorOfClass` "/Game/Core/BP_ScoreReport.BP_ScoreReport_C"))
  (`/Game/Core/BP_ScoreReport.Refresh Scorecard` _returnvalue "NewEnumerator3"))

(fn `Update Score`
  (params (`Given Score` :type Integer))
  (`self.Update ScoreCard` `Given Score`)
  (set `self.TotalScore` (+ `Given Score` (`self.TotalScore`)))
  (bind _aswbp_game_score (cast `/Game/UI/WBP_GameScore` (`WidgetComponent.GetUserWidgetObject` (`self.ScoreWidget`))))
  (`/Game/UI/WBP_GameScore.SetNewScore` _aswbp_game_score (`self.TotalScore`)))

(fn `Update ScoreCard`
  (params (Amount :type Integer))
  (bind _asbp_minigames_handler (cast `/Game/Core/BP_Minigames_Handler` (`GameplayStatics.GetGameInstance`)))
  (`/Game/Core/BP_Minigames_Handler.Submit Score` _asbp_minigames_handler "NewEnumerator3" Amount)
  (bind _returnvalue (`GameplayStatics.GetActorOfClass` "/Game/Core/BP_ScoreReport.BP_ScoreReport_C"))
  (`/Game/Core/BP_ScoreReport.Refresh Scorecard` _returnvalue "NewEnumerator3"))

(fn `UserConstructionScript`)