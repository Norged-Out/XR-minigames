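; Throwable ring for the ring toss game that scores after resting inside a score zone.
; Dropping it from the GrabComponent adds a forward impulse, notifies BP_RTController and plays a toss sound.
; Entering a zone stores its score and enables Tick, which accumulates hold time until OnScored fires; exiting resets this and plays a drop sound.
; Each sound is debounced with a DoOnce and short delay.
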(event `self.ReceiveTick`
  (params (DeltaSeconds :type "Float (single-precision)"))
  (`self.UpdateHoldTime` DeltaSeconds)
  (`self.Try Scoring`))

(event `self.GrabComponent.OnDropped`
  (bind _ring (`self.Ring`))
  (`PrimitiveComponent.AddImpulse` _ring (* (`SceneComponent.GetForwardVector` _ring) 100.0) "None" false)
  (bind _returnvalue (`GameplayStatics.GetActorOfClass` "/Game/RingToss/BP_RTController.BP_RTController_C"))
  (`/Game/RingToss/BP_RTController.On Ring Used` _returnvalue)
  (`self.PlayRingTossSound`))

(event `PlayRingDropSound`
  (`/Engine/EditorBlueprintResources/StandardMacros.DoOnce` false :!label _label
    (:`Completed`
      (`GameplayStatics.PlaySoundAtLocation` "/Game/Audio/S_RingDropped.S_RingDropped" (`self.K2_GetActorLocation`) (struct) 1.0 1.0 0.0 null null null null)
      (`KismetSystemLibrary.Delay` 0.3)
      (goto _label :!via `Reset`))))

(event `PlayRingScoredSound`
  (`/Engine/EditorBlueprintResources/StandardMacros.DoOnce` false :!label _label_2
    (:`Completed`
      (`GameplayStatics.PlaySoundAtLocation` "/Game/Audio/S_RingScored.S_RingScored" (`self.K2_GetActorLocation`) (struct) 1.0 1.0 0.0 null null null null)
      (`KismetSystemLibrary.Delay` 0.3)
      (goto _label_2 :!via `Reset`))))

(event `PlayRingTossSound`
  (`/Engine/EditorBlueprintResources/StandardMacros.DoOnce` false :!label _label_3
    (:`Completed`
      (`GameplayStatics.PlaySoundAtLocation` "/Game/Audio/S_RingTossSound.S_RingTossSound" (`self.K2_GetActorLocation`) (struct) 1.0 1.0 0.0 null null null null)
      (`KismetSystemLibrary.Delay` 0.3)
      (goto _label_3 :!via `Reset`))))

(fn `Enter Score Zone`
  (params (currScore :type Integer))
  (set `self.bInsideZone` true)
  (set `self.Score` currScore)
  (`self.SetActorTickEnabled` true))

(fn `Exit Score Zone`
  (set `self.bInsideZone` false)
  (set `self.holdTime` 0.0)
  (set `self.Score` 0)
  (`self.SetActorTickEnabled` false)
  (`self.PlayRingDropSound`))

(fn `Try Scoring`
  (if (>= (`self.holdTime`) 1.5)
    (set `self.bHasScored` true)
    (`self.OnScored` (`self.Score`))
    (`self.SetActorTickEnabled` false)
    (`self.PlayRingScoredSound`)))

(fn `UpdateHoldTime`
  (params (DeltaSeconds :type "Float (double-precision)"))
  (if (and (`self.bInsideZone`) (not (`self.bHasScored`)))
    (set `self.holdTime` (+ DeltaSeconds (`self.holdTime`)))))

(fn `UserConstructionScript`
  (`PrimitiveComponent.SetMaterial` (`self.Ring`) 0 (`self.Mat`)))