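; A bowling ball Blueprint that launches itself when released from a grab and uses up one of the player's chances.
; On the first drop only, it enables physics on its mesh and applies an impulse along the mesh's forward vector, scaled by a throw strength.
; It then finds the bowling controller in the level to consume a chance and sets a short lifespan so the ball removes itself.
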(event `self.Grab.OnDropped`
  (bind _staticmesh (`self.StaticMesh`))
  (if (not (`self.bHasThrown`))
    (set `self.bHasThrown` true)
    (`PrimitiveComponent.SetSimulatePhysics` _staticmesh true)
    (`PrimitiveComponent.AddImpulse` _staticmesh (* (`SceneComponent.GetForwardVector` _staticmesh) (`self.ThrowStrength`)) "None" false)
    (bind _returnvalue (`GameplayStatics.GetActorOfClass` "/Game/Bowling/BP_BowlingController.BP_BowlingController_C"))
    (`/Game/Bowling/BP_BowlingController.Consume Chance` _returnvalue)
    (`self.SetLifeSpan` 7.0)))

(fn `UserConstructionScript`)