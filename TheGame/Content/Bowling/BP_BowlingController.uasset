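; Bowling minigame controller that starts a game when an XR pawn enters its start zone, showing the score widget only while the pawn is inside.
; Starting resets the score and spawns a triangular pin rack from nested row loops.
; UpdateScore feeds the widget and the carnival player state's shoot-cups score.
; Cup-shooter leftovers remain: gun spawning never runs, yet EndGame still expires the gun while clearing spawned actors.
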(event `self.StartZone.OnComponentBeginOverlap`
  (params (OverlappedComponent :type "PrimitiveComponent Object Reference") (OtherActor :type "Actor Object Reference") (OtherComp :type "PrimitiveComponent Object Reference") (OtherBodyIndex :type Integer) (bFromSweep :type Boolean) (SweepResult :type "HitResult Structure (by ref)"))
  (cast `/Game/XRFramework/Blueprints/BP_XRPawn` OtherActor)
  (set `self.bPlayerInRange` true)
  (`SceneComponent.SetVisibility` (`self.ScoreWidget`) true false)
  (if (not (`self.bGameActive`))
    (`self.Start Game`)))

(event `self.StartZone.OnComponentEndOverlap`
  (params (OverlappedComponent :type "PrimitiveComponent Object Reference") (OtherActor :type "Actor Object Reference") (OtherComp :type "PrimitiveComponent Object Reference") (OtherBodyIndex :type Integer))
  (cast `/Game/XRFramework/Blueprints/BP_XRPawn` OtherActor)
  (set `self.bPlayerInRange` false)
  (`SceneComponent.SetVisibility` (`self.ScoreWidget`) false false))

(fn `Display Message`
  (params (inText :type Text))
  (bind _aswbp_game_score (cast `/Game/UI/WBP_GameScore` (`WidgetComponent.GetUserWidgetObject` (`self.ScoreWidget`))))
  (`/Game/UI/WBP_GameScore.SetMessage` _aswbp_game_score inText))

(fn `End Game`
  (bind _spawnedcups (`self.SpawnedCups`))
  (set `self.bGameActive` false)
  (`self.SetLifeSpan` (`self.Gun`) 2.0)
  (`self.Display Message` "Game Over")
  (for _array_element _spawnedcups
    (`self.K2_DestroyActor` _array_element))
  (`KismetArrayLibrary.Array_Clear` _spawnedcups))

(fn `Spawn Cups`
  (bind _hspacing (`self.hSpacing`))
  (bind _hspacing_2 (`self.hSpacing`))
  (bind _returnvalue (- (`self.RowCount`) 1))
  (for _index (range (+ _returnvalue 1))
    (bind _returnvalue_2 (- _returnvalue _index))
    (for _index_2 (range (+ _returnvalue_2 1))
      (for _index_3 (range (+ _returnvalue_2 1))
        (bind _returnvalue_3 (`|SpawnActorFromClass` "/Game/Bowling/BP_Cup.BP_Cup_C" (`KismetMathLibrary.MakeTransform` (`KismetMathLibrary.MakeVector` (+ (- (* _index_2 _hspacing) (/ (* _hspacing (- (- (`self.RowCount`) _index) 1)) 2.0)) (.x (.location (`SceneComponent.K2_GetComponentToWorld` (`self.CupSpawnPoint`))))) (+ (- (* _index_3 _hspacing_2) (/ (* _hspacing_2 (- (- (`self.RowCount`) _index) 1)) 2.0)) (.y (.location (`SceneComponent.K2_GetComponentToWorld` (`self.CupSpawnPoint`))))) (+ (* _index (`self.vSpacing`)) (.z (.location (`SceneComponent.K2_GetComponentToWorld` (`self.CupSpawnPoint`)))))) (.rotation (`SceneComponent.K2_GetComponentToWorld` (`self.CupSpawnPoint`))) (.scale (`SceneComponent.K2_GetComponentToWorld` (`self.CupSpawnPoint`)))) "Undefined" "MultiplyWithRoot" null null))
        (`KismetArrayLibrary.Array_Add` (`self.SpawnedCups`) _returnvalue_3)))))

(fn `Spawn Gun`
  (bind _returnvalue (`|SpawnActorFromClass` "/Game/Bowling/BP_CupShooter.BP_CupShooter_C" (`KismetMathLibrary.MakeTransform` (.location (`SceneComponent.K2_GetComponentToWorld` (`self.GunSpawnPoint`))) (struct :`Pitch` 90.0 :`Yaw` 180.0) (.scale (`SceneComponent.K2_GetComponentToWorld` (`self.GunSpawnPoint`)))) "Undefined" "MultiplyWithRoot" null null))
  (bind _output_get (set `self.Gun` _returnvalue))
  (add `/Game/Bowling/BP_CupShooter.OnOutOfAmmo` _output_get (`|CreateDelegate` :!event `End Game`)))

(fn `Spawn Pins`
  (bind _hspacing (`self.hSpacing`))
  (for _index (range (`self.RowCount`))
    (for _index_2 (range (+ _index 1))
      (bind _returnvalue (`|SpawnActorFromClass` "/Game/Bowling/BP_Cup.BP_Cup_C" (`KismetMathLibrary.MakeTransform` (`KismetMathLibrary.MakeVector` (+ (- (* _index_2 _hspacing) (/ (* _index _hspacing) 2.0)) (.x (.location (`SceneComponent.K2_GetComponentToWorld` (`self.CupSpawnPoint`))))) (- (.y (.location (`SceneComponent.K2_GetComponentToWorld` (`self.CupSpawnPoint`)))) (* _index (`self.hSpacing`))) (.z (.location (`SceneComponent.K2_GetComponentToWorld` (`self.CupSpawnPoint`))))) (.rotation (`SceneComponent.K2_GetComponentToWorld` (`self.CupSpawnPoint`))) (.scale (`SceneComponent.K2_GetComponentToWorld` (`self.CupSpawnPoint`)))) "Undefined" "MultiplyWithRoot" null null))
      (`KismetArrayLibrary.Array_Add` (`self.SpawnedCups`) _returnvalue))))

(fn `Start Game`
  (set `self.bGameActive` true)
  (set `self.TotalScore` 0)
  (`self.Display Message` "Bowling")
  (`self.Spawn Pins`))

(fn `Update Score`
  (params (givenScore :type Integer))
  (`self.Update ScoreCard` givenScore)
  (set `self.TotalScore` (+ givenScore (`self.TotalScore`)))
  (bind _aswbp_game_score (cast `/Game/UI/WBP_GameScore` (`WidgetComponent.GetUserWidgetObject` (`self.ScoreWidget`))))
  (`/Game/UI/WBP_GameScore.SetNewScore` _aswbp_game_score (`self.TotalScore`)))

(fn `Update ScoreCard`
  (params (Amount :type Integer))
  (bind _asbp_carnival_player_state (cast `/Game/Core/BP_CarnivalPlayerState` (`Controller.PlayerState` (`GameplayStatics.GetPlayerController` 0))))
  (`/Game/Core/BP_CarnivalPlayerState.AddShootCupsScore` _asbp_carnival_player_state Amount))

(fn `UserConstructionScript`)