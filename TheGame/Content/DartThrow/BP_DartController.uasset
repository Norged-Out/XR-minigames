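; Controller for a carnival dart-throw minigame in XR, which starts when the pawn enters the start zone, also showing the score widget.
; BeginPlay spawns a target and a looping timer for spawning randomly colored balloons at two spawners.
; Starting resets the score, spawns a dart gun and binds its out-of-ammo event and the target's hit event.
; Scoring updates the widget and carnival player state; ending expires the gun and shows Game Over.
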(event `self.StartZone.OnComponentBeginOverlap`
  (params (OverlappedComponent :type "PrimitiveComponent Object Reference") (OtherActor :type "Actor Object Reference") (OtherComp :type "PrimitiveComponent Object Reference") (OtherBodyIndex :type Integer) (bFromSweep :type Boolean) (SweepResult :type "HitResult Structure (by ref)"))
  (cast `/Game/XRFramework/Blueprints/BP_XRPawn` OtherActor)
  (set `self.bPlayerInRange` true)
  (`SceneComponent.SetVisibility` (`self.ScoreWidget`) true false)
  (if (not (`self.bGameActive`))
    (`self.Start Game`)))

(event `self.StartZone.OnComponentEndOverlap`
  (params (OverlappedComponent :type "PrimitiveComponent Object Reference") (OtherActor :type "Actor Object Reference") (OtherComp :type "PrimitiveComponent Object Reference") (OtherBodyIndex :type Integer))
  (cast `/Game/XRFramework/Blueprints/BP_XRPawn` OtherActor)
  (set `self.bPlayerInRange` false)
  (`SceneComponent.SetVisibility` (`self.ScoreWidget`) false false))

(event `self.ReceiveBeginPlay`
  (`|SpawnActorFromClass` "/Game/DartThrow/BP_Target.BP_Target_C" (`SceneComponent.K2_GetComponentToWorld` (`self.TargetSpawnPoint`)) "Undefined" "MultiplyWithRoot" null null)
  (`KismetSystemLibrary.K2_SetTimerDelegate` (`|CreateDelegate` :!event `SpawnBalloon`) 5.0 true))

(event `SpawnBalloon`
  (bind _returnvalue (`|SpawnActorFromClass` "/Game/DartThrow/BP_Balloon.BP_Balloon_C" (`SceneComponent.K2_GetComponentToWorld` (`self.LeftBalloonSpawner`)) "Undefined" "MultiplyWithRoot" null (select `int` (`KismetMathLibrary.RandomIntegerInRange` 0 5) :`0` "/Game/Assets/Balloon/MI_Balloon_Black.MI_Balloon_Black" :`1` "/Game/Assets/Balloon/MI_Balloon_Blue.MI_Balloon_Blue" :`2` "/Game/Assets/Balloon/MI_Balloon_Green.MI_Balloon_Green" :`3` "/Game/Assets/Balloon/MI_Balloon_Red.MI_Balloon_Red" :`4` "/Game/Assets/Balloon/MI_Balloon_White.MI_Balloon_White" :`5` "/Game/Assets/Balloon/MI_Balloon_Yellow.MI_Balloon_Yellow" :!type "MaterialInstance Object Reference") null))
  (add `/Game/DartThrow/BP_Balloon.OnTargetHit` _returnvalue (`|CreateDelegate` :!event `Update Score`))
  (bind _returnvalue_2 (`|SpawnActorFromClass` "/Game/DartThrow/BP_Balloon.BP_Balloon_C" (`SceneComponent.K2_GetComponentToWorld` (`self.RightBalloonSpawner`)) "Undefined" "MultiplyWithRoot" null (select `int` (`KismetMathLibrary.RandomIntegerInRange` 0 5) :`0` "/Game/Assets/Balloon/MI_Balloon_Black.MI_Balloon_Black" :`1` "/Game/Assets/Balloon/MI_Balloon_Blue.MI_Balloon_Blue" :`2` "/Game/Assets/Balloon/MI_Balloon_Green.MI_Balloon_Green" :`3` "/Game/Assets/Balloon/MI_Balloon_Red.MI_Balloon_Red" :`4` "/Game/Assets/Balloon/MI_Balloon_White.MI_Balloon_White" :`5` "/Game/Assets/Balloon/MI_Balloon_Yellow.MI_Balloon_Yellow" :!type "MaterialInstance Object Reference") null))
  (add `/Game/DartThrow/BP_Balloon.OnTargetHit` _returnvalue_2 (`|CreateDelegate` :!event `Update Score`)))

(fn `Display Message`
  (params (inText :type Text))
  (bind _aswbp_game_score (cast `/Game/UI/WBP_GameScore` (`WidgetComponent.GetUserWidgetObject` (`self.ScoreWidget`))))
  (`/Game/UI/WBP_GameScore.SetMessage` _aswbp_game_score inText))

(fn `End Game`
  (set `self.bGameActive` false)
  (`self.SetLifeSpan` (`self.Gun`) 2.0)
  (`self.Display Message` "Game Over"))

(fn `Spawn Gun`
  (bind _returnvalue (`|SpawnActorFromClass` "/Game/DartThrow/BP_DartGun.BP_DartGun_C" (`KismetMathLibrary.MakeTransform` (.location (`SceneComponent.K2_GetComponentToWorld` (`self.GunSpawnPoint`))) (struct :`Pitch` 90.0 :`Yaw` 180.0) (.scale (`SceneComponent.K2_GetComponentToWorld` (`self.GunSpawnPoint`)))) "Undefined" "MultiplyWithRoot" null null))
  (bind _output_get (set `self.Gun` _returnvalue))
  (add `/Game/DartThrow/BP_DartGun.OnOutOfAmmo` _output_get (`|CreateDelegate` :!event `End Game`)))

(fn `Start Game`
  (set `self.bGameActive` true)
  (set `self.TotalScore` 0)
  (`self.Display Message` "Dart Throw")
  (`self.Spawn Gun`)
  (bind _returnvalue (`GameplayStatics.GetActorOfClass` "/Game/DartThrow/BP_Target.BP_Target_C"))
  (add `/Game/DartThrow/BP_Target.OnTargetHit` _returnvalue (`|CreateDelegate` :!event `Update Score`)))

(fn `Update Score`
  (params (givenScore :type Integer))
  (`self.Update ScoreCard` givenScore)
  (set `self.TotalScore` (+ givenScore (`self.TotalScore`)))
  (bind _aswbp_game_score (cast `/Game/UI/WBP_GameScore` (`WidgetComponent.GetUserWidgetObject` (`self.ScoreWidget`))))
  (`/Game/UI/WBP_GameScore.SetNewScore` _aswbp_game_score (`self.TotalScore`)))

(fn `Update ScoreCard`
  (params (Amount :type Integer))
  (bind _asbp_carnival_player_state (cast `/Game/Core/BP_CarnivalPlayerState` (`Controller.PlayerState` (`GameplayStatics.GetPlayerController` 0))))
  (`/Game/Core/BP_CarnivalPlayerState.AddDartThrowScore` _asbp_carnival_player_state Amount))

(fn `UserConstructionScript`)