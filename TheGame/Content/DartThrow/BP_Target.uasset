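; BP_Target is the dartboard for the dart throw game, reporting the score of each ring a dart hits.
; On BeginPlay it binds a hit handler to every static mesh under Targets.
; Hits from BP_Dart_New broadcast OnTargetHit with the score, read as an integer from that mesh's first component tag.
; A DoOnce with a short delayed reset throttles the hit sound, but not the scoring.
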(event `self.ReceiveBeginPlay`
  (for _array_element (`SceneComponent.GetChildrenComponents` (`self.Targets`) false)
    (bind _asstatic_mesh_component (cast `StaticMeshComponent` _array_element))
    (add `PrimitiveComponent.OnComponentHit` _asstatic_mesh_component (delegate `SendScore`))))

(event `SendScore`
  (params (HitComponent :type "PrimitiveComponent Object Reference") (OtherActor :type "Actor Object Reference") (OtherComp :type "PrimitiveComponent Object Reference") (NormalImpulse :type "Vector Structure") (Hit :type "HitResult Structure (by ref)"))
  (cast `/Game/DartThrow/BP_Dart_New` OtherActor)
  (`self.OnTargetHit` (`self.Get Score Tag` HitComponent))
  (`self.PlayHitSound`))

(event `PlayHitSound`
  (`/Engine/EditorBlueprintResources/StandardMacros.DoOnce` false :!label _label
    (:`Completed`
      (`GameplayStatics.PlaySoundAtLocation` "/Game/Audio/S_DartHit.S_DartHit" (`self.K2_GetActorLocation`) (struct) 1.0 1.0 0.0 null null null null)
      (`KismetSystemLibrary.Delay` 0.3)
      (goto _label :!via `Reset`))))

(fn `Get Score Tag`
  (params (Ring :type "ActorComponent Object Reference"))
  (returns (ReturnValue :type Integer))
  (return (`KismetStringLibrary.Conv_StringToInt` (`KismetStringLibrary.Conv_NameToString` (`|GetArrayItem` (`ActorComponent.ComponentTags` Ring))))))

(fn `UserConstructionScript`)