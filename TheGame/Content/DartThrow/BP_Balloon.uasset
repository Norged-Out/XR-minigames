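; Balloon target for the dart-throw game that drifts steadily upward every tick.
; When a BP_Dart overlaps the balloon component, it fires OnTargetHit with a fixed score, plays a pop sound and destroys itself.
; The pop sound is gated by a DoOnce with a short delayed reset.
; GetScoreTag reads an integer from the component's first tag, but the hit logic here does not use it.
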(event `self.Balloon.OnComponentBeginOverlap`
  (params (OverlappedComponent :type "PrimitiveComponent Object Reference") (OtherActor :type "Actor Object Reference") (OtherComp :type "PrimitiveComponent Object Reference") (OtherBodyIndex :type Integer) (bFromSweep :type Boolean) (SweepResult :type "HitResult Structure (by ref)"))
  (cast `/Game/DartThrow/BP_Dart` OtherActor)
  (`self.OnTargetHit` 20)
  (`self.BalloonPop`)
  (`self.K2_DestroyActor`))

(event `self.ReceiveTick`
  (params (DeltaSeconds :type "Float (single-precision)"))
  (bind _balloon (`self.Balloon`))
  (bind (_returnvalue_x _returnvalue_y _returnvalue_z) (`KismetMathLibrary.BreakVector` (`SceneComponent.K2_GetComponentLocation` _balloon)))
  (`SceneComponent.K2_SetWorldLocation` _balloon (`KismetMathLibrary.MakeVector` _returnvalue_x _returnvalue_y (+ _returnvalue_z (* DeltaSeconds 20.0))) false false))

(event `BalloonPop`
  (`/Engine/EditorBlueprintResources/StandardMacros.DoOnce` false :!label _label
    (:`Completed`
      (`GameplayStatics.PlaySoundAtLocation` "/Game/Audio/A_HitBalloon.A_HitBalloon" (`self.K2_GetActorLocation`) (struct) 1.0 1.0 0.0 null null null null)
      (`KismetSystemLibrary.Delay` 0.3)
      (goto _label :!via `Reset`))))

(fn `Get Score Tag`
  (returns (ReturnValue :type Integer))
  (return (`KismetStringLibrary.Conv_StringToInt` (`KismetStringLibrary.Conv_NameToString` (`|GetArrayItem` (`ActorComponent.ComponentTags` (`self.Balloon`)))))))

(fn `UserConstructionScript`)