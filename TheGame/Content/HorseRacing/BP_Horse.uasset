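; BP_Horse is the data actor for one horse in a horse racing game, tracking its ID, race progress, win count and betting odds.
; Reset clears progress and recalculates odds, while Increment advances progress by one and Win adds to the win count.
; GetOdds returns flat odds of 2 for five or fewer games, then scales linearly from BestOdds down to 1 as win rate rises.
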(fn `GetOdds`
  (params (n_games :type Integer) (best_odds :type Integer))
  (returns (Odds :type "Float (double-precision)"))
  (if (<= n_games 5)
    (return 2.0) ; Return straight odds of 2 if < 6 games played
    (else
      (return (- best_odds (* (/ (`self.n_wins`) n_games) (+ best_odds -1)))))))

(fn `Increment`
  (returns (NewProgress :type Integer))
  (bind _output_get (set `self.progress` (+ (`self.progress`) 1)))
  (return _output_get))

(fn `Reset`
  (params (nGames :type Integer) (BestOdds :type Integer))
  (set `self.progress` 0)
  (bind _odds (`self.GetOdds` nGames BestOdds))
  (set `self.odds` _odds))

(fn `Set_ID`
  (params (ID :type Integer))
  (set `self.id` ID))

(fn `UserConstructionScript`)

(fn `Win`
  (set `self.n_wins` (+ (`self.n_wins`) 1)))