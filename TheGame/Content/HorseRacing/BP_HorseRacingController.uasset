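; Controller for a horse-racing betting minigame that runs the race, tracks the player's balance and bet, and feeds the UI widget.
; BeginPlay spawns BP_Horse actors into five slots, and StartGame deducts the wager.
; While running, a time-modulo gate on Tick advances a random horse and refreshes progress.
; Reaching WinScore resets horses, updates displayed odds, and pays wager plus odds if the selected horse won.
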(event `self.ReceiveBeginPlay`
  (for _index (range 6)
    (bind _returnvalue (`|SpawnActorFromClass` "/Game/HorseRacing/BP_Horse.BP_Horse_C" (`self.GetTransform`) "Undefined" "MultiplyWithRoot" null null))
    (switch `int` _index
      (:`Default`
        (set `self.H4` _returnvalue))
      (:`0`
        (set `self.H0` _returnvalue))
      (:`1`
        (set `self.H1` _returnvalue))
      (:`2`
        (set `self.H2` _returnvalue))
      (:`3`
        (set `self.H3` _returnvalue)))))

(event `self.ReceiveTick`
  (params (DeltaSeconds :type "Float (single-precision)"))
  (if (`self.running`)
    (if (<= (mod (`GameplayStatics.GetTimeSeconds`) (`self.secsBetweenTicks`)) 0.01)
      (bind _randomhorse (`self.GetRandomHorse`))
      (bind _newprogress (`/Game/HorseRacing/BP_Horse.Increment` _randomhorse))
      (`self.UpdateUI`)
      (if (>= _newprogress (`self.WinScore`))
        (`self.EndGame`)
        (bind _horse (`self.GetHorseByID` (`self.SelectedHorse`)))
        (`/Game/HorseRacing/BP_Horse.Win` _randomhorse)
        (if (== _randomhorse _horse)
          (`self.EarnWinnings`))))))

(event `StartGame`
  (params (BetVal :type "Float (double-precision)"))
  (set `self.running` true)
  (`self.PlaceBet` BetVal))

(event `EndGame`
  (bind _h0 (`self.H0`))
  (bind _n_games (`self.n_games`))
  (bind _bestodds (`self.BestOdds`))
  (bind _h1 (`self.H1`))
  (bind _h2 (`self.H2`))
  (bind _h3 (`self.H3`))
  (bind _h4 (`self.H4`))
  (set `self.n_games` (+ _n_games 1))
  (`/Game/HorseRacing/BP_Horse.Reset` _h0 _n_games _bestodds)
  (`/Game/HorseRacing/BP_Horse.Reset` _h1 _n_games _bestodds)
  (`/Game/HorseRacing/BP_Horse.Reset` _h2 _n_games _bestodds)
  (`/Game/HorseRacing/BP_Horse.Reset` _h3 _n_games _bestodds)
  (`/Game/HorseRacing/BP_Horse.Reset` _h4 _n_games _bestodds)
  (bind _ashorse_racing_ui (cast `/Game/UI/Horse_Racing_UI` (`WidgetComponent.GetUserWidgetObject` (`self.GameWidget`))))
  (`/Game/UI/Horse_Racing_UI.UpdateUIOdds` _ashorse_racing_ui (`/Game/HorseRacing/BP_Horse.odds` _h0) (`/Game/HorseRacing/BP_Horse.odds` _h1) (`/Game/HorseRacing/BP_Horse.odds` _h2) (`/Game/HorseRacing/BP_Horse.odds` _h3) (`/Game/HorseRacing/BP_Horse.odds` _h4))
  (set `self.running` false))

(fn `EarnWinnings`
  (set `self.balance` (+ (`self.balance`) (+ (`self.wagerVal`) (`self.CurrentOdds`)))))

(fn `GetHorseByID`
  (params (ID :type Integer))
  (returns (Horse :type "/Game/HorseRacing/BP_Horse Object Reference"))
  (switch `int` ID
    (:`Default`
      (return (`self.H4`)))
    (:`0`
      (return (`self.H0`)))
    (:`1`
      (return (`self.H1`)))
    (:`2`
      (return (`self.H2`)))
    (:`3`
      (return (`self.H3`)))))

(fn `GetRandomHorse`
  (returns (RandomHorse :type "/Game/HorseRacing/BP_Horse Object Reference"))
  (locals (val :type Integer))
  (bind _output_get (set `local.val` (`KismetMathLibrary.RandomInteger` 5)))
  (if (== _output_get 0)
    (return (`self.H0`))
    (elif (== _output_get 1)
      (return (`self.H1`))
      (elif (== _output_get 2)
        (return (`self.H2`))
        (elif (== _output_get 3)
          (return (`self.H3`))
          (else
            (return (`self.H4`))))))))

(fn `PlaceBet`
  (params (Value :type "Float (double-precision)"))
  (set `self.balance` (- (`self.balance`) Value))
  (set `self.wagerVal` Value))

(fn `SelectHorse`
  (params (HorseID :type Integer))
  (bind _output_get (set `self.SelectedHorse` HorseID))
  (switch `int` _output_get
    (:`Default`
      (set `self.CurrentOdds` (`/Game/HorseRacing/BP_Horse.odds` (`self.H4`))))
    (:`0`
      (set `self.CurrentOdds` (`/Game/HorseRacing/BP_Horse.odds` (`self.H0`))))
    (:`1`
      (set `self.CurrentOdds` (`/Game/HorseRacing/BP_Horse.odds` (`self.H1`))))
    (:`2`
      (set `self.CurrentOdds` (`/Game/HorseRacing/BP_Horse.odds` (`self.H2`))))
    (:`3`
      (set `self.CurrentOdds` (`/Game/HorseRacing/BP_Horse.odds` (`self.H3`))))))

(fn `UpdateUI`
  (bind _ashorse_racing_ui (cast `/Game/UI/Horse_Racing_UI` (`WidgetComponent.GetUserWidgetObject` (`self.GameWidget`))))
  (`/Game/UI/Horse_Racing_UI.Update` _ashorse_racing_ui (`/Game/HorseRacing/BP_Horse.progress` (`self.H0`)) (`/Game/HorseRacing/BP_Horse.progress` (`self.H1`)) (`/Game/HorseRacing/BP_Horse.progress` (`self.H2`)) (`/Game/HorseRacing/BP_Horse.progress` (`self.H3`)) (`/Game/HorseRacing/BP_Horse.progress` (`self.H4`))))

(fn `UserConstructionScript`)