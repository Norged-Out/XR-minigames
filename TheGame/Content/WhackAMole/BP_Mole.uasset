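; BP_Mole is a whack-a-mole target that awards points when struck by the hammer.
; On BeginPlay it clears its hit flag and caches its starting location plus a hide location slightly below it.
; HitByHammer sets the hit flag, prints a debug message, passes its Score to the BP_WMController found in the level, then snaps the mole down to the hide location.
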(event `self.ReceiveBeginPlay`
  ; Setup
  (set `self.bHasBeenHit` false)
  (bind _output_get (set `self.MainLoc` (`self.K2_GetActorLocation`)))
  (set `self.HideLoc` (`KismetMathLibrary.MakeVector` (.x _output_get) (.y _output_get) (- (.z _output_get) 10.0))))

(fn `Hit By Hammer`
  (set `self.bHasBeenHit` true)
  (`KismetSystemLibrary.PrintString` "Hammer-chan hit me!")
  (bind _returnvalue (`GameplayStatics.GetActorOfClass` "/Game/WhackAMole/BP_WMController.BP_WMController_C"))
  (`/Game/WhackAMole/BP_WMController.Update Score` _returnvalue (`self.Score`))
  (`self.K2_SetActorLocation` (`self.HideLoc`)))

(fn `UserConstructionScript`)