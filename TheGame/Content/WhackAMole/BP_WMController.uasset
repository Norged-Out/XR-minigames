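; Whack-a-mole game controller that starts a timed, multi-round game when the XR pawn enters its start zone.
; StartGame spawns a hammer, then timers alternate StartRound and EndRound to spawn and clear moles until MaxRounds ends the game.
; Moles spawn at random transforms cached from the Holes child components on BeginPlay.
; A score widget, visible while the player is in the zone, shows round messages and the score from UpdateScore.
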(event `self.StartZone.OnComponentBeginOverlap`
  (params (OverlappedComponent :type "PrimitiveComponent Object Reference") (OtherActor :type "Actor Object Reference") (OtherComp :type "PrimitiveComponent Object Reference") (OtherBodyIndex :type Integer) (bFromSweep :type Boolean) (SweepResult :type "HitResult Structure (by ref)"))
  (cast `/Game/XRFramework/Blueprints/BP_XRPawn` OtherActor)
  (set `self.bPlayerInRange` true)
  (`SceneComponent.SetVisibility` (`self.ScoreWidget`) true false)
  (if (not (`self.bGameActive`))
    (`self.Start Game`)))

(event `self.StartZone.OnComponentEndOverlap`
  (params (OverlappedComponent :type "PrimitiveComponent Object Reference") (OtherActor :type "Actor Object Reference") (OtherComp :type "PrimitiveComponent Object Reference") (OtherBodyIndex :type Integer))
  (cast `/Game/XRFramework/Blueprints/BP_XRPawn` OtherActor)
  (set `self.bPlayerInRange` false)
  (`SceneComponent.SetVisibility` (`self.ScoreWidget`) false false))

(event `self.ReceiveBeginPlay`
  (for _array_element (`SceneComponent.GetChildrenComponents` (`self.Holes`) true)
    (`KismetArrayLibrary.Array_Add` (`self.Mole Spawn Points`) (`SceneComponent.K2_GetComponentToWorld` _array_element)))
  (`KismetSystemLibrary.PrintText` "Mole Array Filled"))

(fn `Display Message`
  (params (`In Text` :type Text))
  (bind _aswbp_game_score (cast `/Game/UI/WBP_GameScore` (`WidgetComponent.GetUserWidgetObject` (`self.ScoreWidget`))))
  (`/Game/UI/WBP_GameScore.SetMessage` _aswbp_game_score `In Text`))

(fn `End Game`
  (bind _curr_hammer (`self.Curr Hammer`))
  (set `self.bGameActive` false)
  (`self.Display Message` "Game Over")
  (`/Engine/EditorBlueprintResources/StandardMacros.IsValid` _curr_hammer
    (:`Is Valid`
      (`self.K2_DestroyActor` _curr_hammer))))

(fn `End Round`
  (bind _active_moles (`self.Active Moles`))
  (for _array_element _active_moles
    (`/Engine/EditorBlueprintResources/StandardMacros.IsValid` _array_element
      (:`Is Valid`
        (`self.K2_DestroyActor` _array_element))))
  (`KismetArrayLibrary.Array_Clear` _active_moles)
  (if (>= (`self.Curr Round`) (`self.Max Rounds`))
    (`self.End Game`)
    (else
      (`KismetSystemLibrary.K2_SetTimer` null "Start Round" 2.0))))

(fn `Spawn Hammer`
  (bind _returnvalue (`|SpawnActorFromClass` "/Game/WhackAMole/BP_Hammer.BP_Hammer_C" (`KismetMathLibrary.MakeTransform` (.location (`SceneComponent.K2_GetComponentToWorld` (`self.HammerSpawnPoint`))) (struct :`Pitch` 90.0 :`Yaw` 180.0) (.scale (`SceneComponent.K2_GetComponentToWorld` (`self.HammerSpawnPoint`)))) "Undefined" "MultiplyWithRoot" null null))
  (set `self.Curr Hammer` _returnvalue))

(fn `Spawn Moles`
  (locals (`Available Spawn Points` :type "Array of Transform Structure"))
  (bind _returnvalue (`KismetMathLibrary.RandomIntegerInRange` 2 3))
  (bind _available_spawn_points (`local.Available Spawn Points`))
  (bind _returnvalue_2 (`KismetMathLibrary.RandomIntegerInRange` 0 (`KismetArrayLibrary.Array_Length` _available_spawn_points)))
  (set `local.Available Spawn Points` (`self.Mole Spawn Points`))
  (`KismetSystemLibrary.PrintText` (`|FormatText` "Spawning {n} Moles" _returnvalue))
  (for _ (range (+ _returnvalue 1))
    (bind _returnvalue_3 (`|SpawnActorFromClass` "/Game/WhackAMole/BP_Mole.BP_Mole_C" (`KismetArrayLibrary.Array_Get` _available_spawn_points _returnvalue_2) "Undefined" "MultiplyWithRoot" null null))
    (`KismetArrayLibrary.Array_Add` (`self.Active Moles`) _returnvalue_3)
    (`KismetArrayLibrary.Array_Remove` _available_spawn_points _returnvalue_2)))

(fn `Start Game`
  (set `self.bGameActive` true)
  (set `self.Total Score` 0)
  (set `self.Curr Round` 0)
  (`self.Spawn Hammer`)
  (`KismetSystemLibrary.K2_SetTimer` null "Start Round" 5.0))

(fn `Start Round`
  (bind _output_get (set `self.Curr Round` (+ (`self.Curr Round`) 1)))
  (`self.Display Message` (`|FormatText` "Round: {RoundNum}" (`KismetTextLibrary.Conv_IntToText` _output_get)))
  (`self.Spawn Moles`)
  (`KismetSystemLibrary.K2_SetTimer` null "End Round" 5.0))

(fn `Update Score`
  (params (`Given Score` :type Integer))
  (set `self.Total Score` (+ `Given Score` (`self.Total Score`)))
  (bind _aswbp_game_score (cast `/Game/UI/WBP_GameScore` (`WidgetComponent.GetUserWidgetObject` (`self.ScoreWidget`))))
  (`/Game/UI/WBP_GameScore.SetNewScore` _aswbp_game_score (`self.Total Score`)))

(fn `UserConstructionScript`)