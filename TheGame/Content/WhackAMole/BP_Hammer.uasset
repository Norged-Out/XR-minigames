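; BP_Hammer is the hammer for a whack-a-mole game, telling moles when its head strikes them and playing an impact sound.
; On BeginPlay it binds to the Head component's begin-overlap event and ignores any overlapping actor that is not a BP_Mole.
; Each mole overlap calls HitByHammer, while a DoOnce reset after a short delay throttles only the sound, played at the hammer's location.
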(event `self.ReceiveBeginPlay`
  (add `PrimitiveComponent.OnComponentBeginOverlap` (`self.Head`) (delegate `ObjectHit`)))

(event `ObjectHit`
  (params (OverlappedComponent :type "PrimitiveComponent Object Reference") (OtherActor :type "Actor Object Reference") (OtherComp :type "PrimitiveComponent Object Reference") (OtherBodyIndex :type Integer) (bFromSweep :type Boolean) (SweepResult :type "HitResult Structure (by ref)"))
  (bind _asbp_mole (cast `/Game/WhackAMole/BP_Mole` OtherActor))
  (`/Game/WhackAMole/BP_Mole.Hit By Hammer` _asbp_mole)
  (`self.Hammah`))

(event `Hammah`
  (`/Engine/EditorBlueprintResources/StandardMacros.DoOnce` false :!label _label
    (:`Completed`
      (`GameplayStatics.PlaySoundAtLocation` "/Game/Audio/HAMMAH.HAMMAH" (`self.K2_GetActorLocation`) (struct) 1.0 1.0 0.0 null null null null)
      (`KismetSystemLibrary.Delay` 0.3)
      (goto _label :!via `Reset`))))

(fn `UserConstructionScript`)