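; BP_Minigames_Handler tracks scores for the game's minigames, Whack-A-Mole and Bowling.
; SubmitScore switches on the game type to add a score to that game's total, increment its attempt count, and add the score to a shared grand total.
; GetGameStats returns the total and attempt count for the requested game type.
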(fn `GetGameStats`
  (params (`Game Type` :type "/Game/Core/E_GameType Enum" :default "NewEnumerator0"))
  (returns (Total :type Integer) (Attempts :type Integer))
  (switch `/Game/Core/E_GameType` `Game Type`
    (:`NewEnumerator0`
      (return (`self.WAM Total`) (`self.WAM Attempts`)))
    (:`NewEnumerator1`
      (return (`self.Bowling Total`) (`self.Bowling Attempts`)))))

(fn `SubmitScore`
  (params (`Game Type` :type "/Game/Core/E_GameType Enum" :default "NewEnumerator0") (Score :type Integer))
  (locals (`New Score` :type Integer))
  (set `local.New Score` Score)
  (switch `/Game/Core/E_GameType` `Game Type`
    (:`NewEnumerator0`
      (set `self.WAM Total` (+ (`self.WAM Total`) (`local.New Score`)))
      (set `self.WAM Attempts` (+ (`self.WAM Attempts`) 1)))
    (:`NewEnumerator1`
      (set `self.Bowling Total` (+ (`self.Bowling Total`) (`local.New Score`)))
      (set `self.Bowling Attempts` (+ (`self.Bowling Attempts`) 1))))
  (set `self.Grand Total` (+ (`self.Grand Total`) (`local.New Score`))))