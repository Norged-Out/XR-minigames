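; Player state for a carnival game that tracks separate scores for the ring toss, dart throw and shoot cups minigames.
; Each Add function increases its score by an amount, then calls NotifyScoreChanged with that minigame's enum value.
; NotifyScoreChanged is currently an empty stub, so score changes are not broadcast from here.
; GetTotalScore returns the sum of the three scores.
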(fn `AddDartThrowScore`
  (params (Amount :type Integer))
  (set `self.DartThrowScore` (+ Amount (`self.DartThrowScore`)))
  (`self.NotifyScoreChanged` "NewEnumerator1"))

(fn `AddRingTossScore`
  (params (Amount :type Integer))
  (set `self.RingTossScore` (+ Amount (`self.RingTossScore`)))
  (`self.NotifyScoreChanged` "NewEnumerator0"))

(fn `AddShootCupsScore`
  (params (Amount :type Integer))
  (set `self.ShootCupsScore` (+ Amount (`self.ShootCupsScore`)))
  (`self.NotifyScoreChanged` "NewEnumerator2"))

(fn `GetTotalScore`
  (returns (TotalScore :type Integer))
  (return (+ (`self.RingTossScore`) (`self.DartThrowScore`) (`self.ShootCupsScore`))))

(fn `NotifyScoreChanged`
  (params (GameType :type "/Game/Core/E_CarnivalGame Enum" :default "NewEnumerator0")))

(fn `UserConstructionScript`)