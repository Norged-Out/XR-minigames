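; BP_Cup is a target cup in the ShootCups game that awards score once when it is toppled.
; Each Hit call compares the cup mesh's up vector to its starting up vector, accumulating CheckInterval while the tilt meets the threshold and resetting otherwise.
; Reaching the hold time plays hit and falling sounds, guarded by self-resetting DoOnce nodes, then sends the cup's score value to BP_CupController.
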(event `self.ReceiveHit`
  (params (MyComp :type "PrimitiveComponent Object Reference") (Other :type "Actor Object Reference") (OtherComp :type "PrimitiveComponent Object Reference") (bSelfMoved :type Boolean) (HitLocation :type "Vector Structure") (HitNormal :type "Vector Structure") (NormalImpulse :type "Vector Structure") (Hit :type "HitResult Structure (by ref)"))
  (if (`self.bHasScored`)
    _
    (elif (`self.CheckValidDegree`)
      (bind _output_get (set `self.ToppledTime` (+ (`self.ToppledTime`) (`self.CheckInterval`))))
      (if (>= _output_get (`self.ToppleHoldTime`))
        (set `self.bHasScored` true)
        (`self.PlayBallHitSound`)
        (`KismetSystemLibrary.Delay` 0.3)
        (`self.PlayCupFallingDownSound`)
        (bind _returnvalue (`GameplayStatics.GetActorOfClass` "/Game/ShootCups/BP_CupController.BP_CupController_C"))
        (`/Game/ShootCups/BP_CupController.Update Score` _returnvalue (`self.ScoreValue`)))
      (else
        (set `self.ToppledTime` 0.0)))))

(event `self.ReceiveBeginPlay`
  (set `self.StartTransform` (`self.GetTransform`)))

(event `PlayBallHitSound`
  ; Play sound for target hit
  (`/Engine/EditorBlueprintResources/StandardMacros.DoOnce` false :!label _label
    (:`Completed`
      (`GameplayStatics.PlaySoundAtLocation` "/Game/Audio/A_HitTarget_Cue.A_HitTarget_Cue" (`self.K2_GetActorLocation`) (struct) 1.0 1.0 0.0 null null null null)
      (`KismetSystemLibrary.Delay` 0.3)
      (goto _label :!via `Reset`))))

(event `PlayCupFallingDownSound`
  ; Play sound for target hit
  (`/Engine/EditorBlueprintResources/StandardMacros.DoOnce` false :!label _label_2
    (:`Completed`
      (`GameplayStatics.PlaySoundAtLocation` "/Game/Audio/S_CupFalling.S_CupFalling" (`self.K2_GetActorLocation`) (struct) 1.0 1.0 0.0 null null null null)
      (`KismetSystemLibrary.Delay` 0.3)
      (goto _label_2 :!via `Reset`))))

(fn `CheckValidDegree`
  (returns (ReturnValue :type Boolean))
  (return (>= (`KismetMathLibrary.RadiansToDegrees` (`KismetMathLibrary.Acos` (`KismetMathLibrary.FClamp` (`KismetMathLibrary.Dot_VectorVector` (`SceneComponent.GetUpVector` (`self.CupMesh`)) (`KismetMathLibrary.GetUpVector` (.rotation (`self.StartTransform`)))) -1.0))) (`self.ToppleAngleDeg`))))

(fn `UserConstructionScript`)